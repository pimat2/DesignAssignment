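; BP_Brain is the puzzle manager that tracks completion of the Air, Fire and Earth temples and opens the energy wall.
; On BeginPlay it caches the two towers and the energy wall, and check events test the concrete blocks, lit torches and broken vases.
; Each solved temple plays a success sound and increments a counter, with Air and Fire also enabling their tower's ball.
; Completing all three destroys the wall.
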(event `GetEnergyTornado`
  ;[1 1 1] Gets all the necessarry references for the spawning of particles near the tower
  (bind _outactors (`GameplayStatics.GetAllActorsOfClass` "/Game/ElementObjects/BP_EnergyWall.BP_EnergyWall_C"))
  (set `self.EnergyWall` (`|GetArrayItem` _outactors)))

(event `GetFireTower`
  ;[1 1 1] Gets all the necessarry references for the spawning of particles near the tower
  (bind _outactors (`GameplayStatics.GetAllActorsOfClass` "/Game/ObjectBlueprints/BP_SecondTower.BP_SecondTower_C"))
  (set `self.FireTower` (`|GetArrayItem` _outactors)))

(event `GetAirTower`
  ;[1 1 1] Gets all the necessarry references for the spawning of particles near the tower
  (bind _outactors (`GameplayStatics.GetAllActorsOfClass` "/Game/ObjectBlueprints/BP_FirstTower.BP_FirstTower_C"))
  (set `self.AirTower` (`|GetArrayItem` _outactors)))

(event `CheckGreenConcrete`
  ;[1 1 1] Checks for the completion of the Air Temple
  (if (`self.GreenConcrete`)
    (`KismetSystemLibrary.PrintString` "GreenBlockActivated")))

(event `self.ReceiveBeginPlay`
  (`self.GetAirTower`)
  (`self.GetFireTower`)
  (`self.GetEnergyTornado`))

(event `CheckRedConcrete`
  ;[1 1 1] Checks for the completion of the Air Temple
  (if (`self.RedConcrete`)
    (`KismetSystemLibrary.PrintString` "RedBlockActivated")))

(event `self.ReceiveTick`
  (params (DeltaSeconds :type "Float (single-precision)")))

(event `CheckForBoth`
  ;[1 1 1] Checks for the completion of the Air Temple
  (if (and (`self.GreenConcrete`) (`self.RedConcrete`))
    (`KismetSystemLibrary.PrintString` "BothActivated")
    (`GameplayStatics.PlaySoundAtLocation` "/Game/SoundsAndAttenuations/Success_3.Success_3" (`self.K2_GetActorLocation` (`GameplayStatics.GetPlayerController` 0)) (struct) 0.3 1.0 0.0 null null null null)
    (`/Game/ObjectBlueprints/BP_FirstTower.EnableAirBall` (`self.AirTower`))
    (bind _output_get (set `self.CompletedElements` (+ (`self.CompletedElements`) 1)))
    (`KismetSystemLibrary.PrintString` (`KismetStringLibrary.Conv_IntToString` _output_get))
    (`self.CheckElementalConditions`)))

(event `CheckLitTorches`
  ;[1 1 1] Checks for the completion of the Fire Temple
  (if (== (`self.LitTorches`) 3)
    (`KismetSystemLibrary.PrintString` "AllTorchesLit")
    (`GameplayStatics.PlaySoundAtLocation` "/Game/SoundsAndAttenuations/Success_3.Success_3" (`self.K2_GetActorLocation` (`GameplayStatics.GetPlayerController` 0)) (struct) 0.3 1.0 0.0 null null null null)
    (`/Game/ObjectBlueprints/BP_SecondTower.EnableFireball` (`self.FireTower`))
    (bind _output_get (set `self.CompletedElements` (+ (`self.CompletedElements`) 1)))
    (`KismetSystemLibrary.PrintString` (`KismetStringLibrary.Conv_IntToString` _output_get))
    (`self.CheckElementalConditions`)))

(event `CheckBrokenVases`
  ;[1 1 1] Checks for the completion of the Earth Temple
  (if (== (`self.BrokenVases`) 4)
    (`KismetSystemLibrary.PrintString` "AllVasesBroken")
    (`GameplayStatics.PlaySoundAtLocation` "/Game/SoundsAndAttenuations/Success_3.Success_3" (`self.K2_GetActorLocation` (`GameplayStatics.GetPlayerController` 0)) (struct) 0.3 1.0 0.0 null null null null)
    (bind _output_get (set `self.CompletedElements` (+ (`self.CompletedElements`) 1)))
    (`KismetSystemLibrary.PrintString` (`KismetStringLibrary.Conv_IntToString` _output_get))
    (`self.CheckElementalConditions`)))

(event `CheckElementalConditions`
  ;[1 1 1] Checks if all temples are complete
  (if (== (`self.CompletedElements`) 3)
    (`self.K2_DestroyActor` (`self.EnergyWall`))))

(fn `UserConstructionScript`)