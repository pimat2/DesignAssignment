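; Destructible wall actor that loses health from any damage and burns away.
; Each hit subtracts damage from an integer Health, and the burn triggers only when the result is exactly zero.
; It then attaches a fire emitter to the mesh, plays a burning sound at its location, and sets a short lifespan.
; A delay matching that lifespan precedes stopping the sound.
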(event `self.ReceiveTick`
  (params (DeltaSeconds :type "Float (single-precision)")))

(event `self.ReceiveAnyDamage`
  (params (Damage :type "Float (single-precision)") (DamageType :type "DamageType Object Reference") (InstigatedBy :type "Controller Object Reference") (DamageCauser :type "Actor Object Reference"))
  (bind _output_get (set `self.Health` (`KismetMathLibrary.FTrunc` (- (`self.Health`) Damage))))
  (if (== _output_get 0)
    (`GameplayStatics.SpawnEmitterAttached` "/Game/Realistic_Starter_VFX_Pack_Vol2/Particles/Fire/P_Fire_Wall.P_Fire_Wall" (`self.StaticMeshComponent`))
    (bind _returnvalue (`GameplayStatics.SpawnSoundAtLocation` "/Game/SoundsAndAttenuations/Burning_forest_ambiance.Burning_forest_ambiance" (`self.K2_GetActorLocation`) (struct) 1.0 1.0 0.0 "/Game/SoundsAndAttenuations/FireAttenuation.FireAttenuation" null))
    (`self.SetLifeSpan` 5.0)
    (`KismetSystemLibrary.Delay` 5.0)
    (`AudioComponent.Stop` _returnvalue)))

(fn `UserConstructionScript`)