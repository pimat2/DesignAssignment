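; BP_Vase is a breakable vase that reports its destruction to a shared BP_Brain actor.
; On BeginPlay it caches the first BP_Brain found in the level.
; Damage of exactly one fixed amount increments the brain's broken-vase count, prints it and calls CheckBrokenVases.
; It then plays an attenuated glass impact sound and destroys itself after a short delay, with no guard against repeat hits meanwhile.
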(event `self.ReceiveBeginPlay`
  (`self.GetBrainREF`))

(event `GetBrainREF`
  (bind _outactors (`GameplayStatics.GetAllActorsOfClass` "/Game/ObjectBlueprints/BP_Brain.BP_Brain_C"))
  (set `self.BrainREF` (`|GetArrayItem` _outactors)))

(event `self.ReceiveAnyDamage`
  (params (Damage :type "Float (single-precision)") (DamageType :type "DamageType Object Reference") (InstigatedBy :type "Controller Object Reference") (DamageCauser :type "Actor Object Reference"))
  (bind _brainref (`self.BrainREF`))
  (if (== Damage 25.0)
    (bind _output_get (set `/Game/ObjectBlueprints/BP_Brain.BrokenVases` (+ (`/Game/ObjectBlueprints/BP_Brain.BrokenVases` _brainref) 1) _brainref))
    (`KismetSystemLibrary.PrintString` (`KismetStringLibrary.Conv_IntToString` _output_get))
    (`/Game/ObjectBlueprints/BP_Brain.CheckBrokenVases` _brainref)
    (`GameplayStatics.PlaySoundAtLocation` "/Game/SoundsAndAttenuations/Impact_Glass_04.Impact_Glass_04" (`self.K2_GetActorLocation`) (struct) 0.5 1.0 0.0 "/Game/SoundsAndAttenuations/VaseAttenuation.VaseAttenuation" null null null)
    (`KismetSystemLibrary.Delay` 2.0)
    (`self.K2_DestroyActor`)))

(fn `UserConstructionScript`)